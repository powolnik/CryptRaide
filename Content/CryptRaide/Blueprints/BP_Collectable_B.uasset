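; BP_Collectable_B is a collectable that ends the game when picked up.
; Its Collected event runs once, calls the parent logic and alters the RotatingMovement spin on all three axes.
; After a delay it shows the EndGame widget with a cursor and UI-only input.
; After a second delay it removes the widget, restores game input and opens Level_WorkInProgress.
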(event EventCollected
  (bind _returnvalue (Game|GetPlayerController 0))
  (bind _returnvalue_2 (Game|GetPlayerController 0))
  (bind _rotatingmovement (Variables|Default|GetRotatingMovement))
  (Utilities|FlowControl|DoOnce false
    (:Completed
      (|CallParentFunction)
      (Variables|/Script/Engine.RotatingMovementComponent|SetRotationRate _rotatingmovement (Math|Rotator|MakeRotator (+ (.roll (Variables|/Script/Engine.RotatingMovementComponent|GetRotationRate _rotatingmovement)) 1.8e+02) (+ (.pitch (Variables|/Script/Engine.RotatingMovementComponent|GetRotationRate _rotatingmovement)) -9e+01) (* (.yaw (Variables|/Script/Engine.RotatingMovementComponent|GetRotationRate _rotatingmovement)) 2.0)))
      (Utilities|FlowControl|Delay 4.0)
      (bind _returnvalue_3 (UserInterface|CreateWidget "/Game/CryptRaide/Blueprints/EndGame.EndGame_C"))
      (UserInterface|Viewport|AddtoViewport _returnvalue_3 0)
      (Variables|/Script/Engine.PlayerController|SetbShowMouseCursor _returnvalue true)
      (Input|SetInputModeUIOnly _returnvalue _returnvalue_3 "DoNotLock" false)
      (Utilities|FlowControl|Delay 3.0)
      (Widget|RemovefromParent _returnvalue_3)
      (Input|SetInputModeGameOnly _returnvalue_2 false)
      (Variables|/Script/Engine.PlayerController|SetbShowMouseCursor _returnvalue_2 false)
      (Game|OpenLevel(byName) "Level_WorkInProgress"))))

(fn ConstructionScript)